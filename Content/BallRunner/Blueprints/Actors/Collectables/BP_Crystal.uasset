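; BP_Crystal is a collectable crystal that flies into the player when touched, then disappears.
; On overlap with player pawn 0, it caches its starting location, scale and light intensity, then plays the TL_BlendAlpha timeline.
; Separate timeline tracks lerp it toward the player's live position, shrink it to zero and fade its light.
; The actor destroys itself when the timeline finishes, with no score or pickup count handled here.
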(event Collision|EventActorBeginOverlap
  (params (OtherActor :type Actor%20Object%20Reference))
  (Utilities|IsPlayer OtherActor
    (:True
      (CallFunction|ObjectStartValues)
      (bind (_direction _smoothlerpalpha _scale _lights) (Timeline|TL_BlendAlpha Play)
        (:Update
          (CallFunction|NewLocation _smoothlerpalpha)
          (CallFunction|NewScale _scale)
          (CallFunction|NewLights _lights))
        (:Finished
          (Actor|DestroyActor))))))

(fn ConstructionScript)

(fn NewFunction0
  (params (A :type Vector%20%28by%20ref%29))
  (Class|KismetMathLibrary|VectorSet A 0.0 0.0 0.0))

(fn ObjectStartValues
  (Variables|Default|SetLerpStartLocation (Transformation|GetActorLocation))
  (Variables|Default|SetLerpStartScale (Transformation|GetActorScale3D))
  (Variables|Default|SetLerpStartLights (Variables|/Script/Engine.LightComponentBase|GetIntensity (Variables|Default|GetLight))))

(fn NewLocation
  (params (Alpha :type Float%20%28single-precision%29))
  (Transformation|SetActorLocation (Math|Vector|Lerp(Vector) (Variables|Default|GetLerpStartLocation) (Transformation|GetActorLocation (Game|Player|GetPlayerPawn 0)) Alpha) false false))

(fn NewScale
  (params (Alpha :type Float%20%28single-precision%29))
  (Transformation|SetActorScale3D (Math|Vector|Lerp(Vector) (Variables|Default|GetLerpStartScale) "0, 0, 0" Alpha)))

(fn NewLights
  (params (Alpha :type Float%20%28single-precision%29))
  (Rendering|Components|Light|SetIntensity (Variables|Default|GetLight) (Math|Float|Lerp (Variables|Default|GetLerpStartLights) 0.0 Alpha)))